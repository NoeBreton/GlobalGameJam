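; BP_HeroTest is a hero actor that automatically travels along a referenced spline path from BeginPlay and can die.
; MoveObject scales a timeline's play rate by the completion time and maps its alpha to spline distance, setting location and rotation each update.
; Location is sampled in world space, rotation in local space.
; DeathLogic runs once, stopping the timeline, hiding the mesh and activating the death effect.
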(event `self.ReceiveBeginPlay`
  ;[1 1 1] Begin Play
  (`self.Move Object`))

(event `Move Object`
  (bind _spline (`/Game/Hero/Spline/BP_SplinePath.Spline` (`self.SplinePath`)))
  ;[0 1 0] Move Object (following a spline)
  (set `self.Is Moving ?` true)
  (`TimelineComponent.SetPlayRate` (`self.Move Object T`) (/ 1.0 (`self.Time To Complete (in seconds)`)))
  (bind (_direction _player_movement_timeline) (`Timeline|Move Object T` :!via `PlayFromStart` :!label _label)
    (:`Update`
      (bind _returnvalue (`KismetMathLibrary.Lerp` 0.0 (`SplineComponent.GetSplineLength` (`/Game/Hero/Spline/BP_SplinePath.Spline` (`self.SplinePath`))) _player_movement_timeline))
      (`self.K2_SetActorTransform` (`KismetMathLibrary.MakeTransform` (`SplineComponent.GetLocationAtDistanceAlongSpline` _spline _returnvalue "World") (`SplineComponent.GetRotationAtDistanceAlongSpline` _spline _returnvalue "Local") (`SceneComponent.K2_GetComponentScale` (`self.Mesh`)))))
    (:`Finished`
      (set `self.Is Moving ?` false))))

(event `Stop Hero Moving`
  ;[0 1 0] Move Object (following a spline)
  (goto _label :!via `Stop`))

(event `Death Logic`
  ;[0 0.992 0] Death Logic
  (if (not (`self.Is Dead ?`))
    (set `self.Is Dead ?` true)
    (`self.Stop Hero Moving`)
    (`SceneComponent.SetVisibility` (`self.Mesh`) false false)
    (`ActorComponent.SetActive` (`self.NS Death FX`) true false)))

(fn `UserConstructionScript`)