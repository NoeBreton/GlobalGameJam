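; BishopKnight boss Blueprint that runs a scripted dialogue with a slime, with comedic sound stingers.
; BeginPlay creates the WBP_Dialogue widget, gives it input focus and fires StartDialogueEvent.
; Each call plays any sound tied to the next row, uses OrderArr to show boss, slime or both portraits, then advances the NPCText row.
; Past the last line the widget is removed, and a level opens if the row has reached the final threshold.
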(event `self.ReceiveBeginPlay`
  (bind _returnvalue (`GameplayStatics.GetActorOfClass` "/Game/ThirdPerson/Blueprints/BP_ThirdPersonCharacter.BP_ThirdPersonCharacter_C"))
  (bind _asplayer_controller (cast `PlayerController` (`Pawn.GetController` _returnvalue)))
  (bind _returnvalue_2 (`|CreateWidget` "/Game/Level_Game/WBP_Dialogue.WBP_Dialogue_C" _asplayer_controller))
  (`UserWidget.AddToViewport` _returnvalue_2 0)
  (bind _output_get (set `self.DialogueUI` _returnvalue_2))
  (`WidgetBlueprintLibrary.SetInputMode_GameAndUIEx` (`GameplayStatics.GetPlayerController` 0) _output_get)
  (`self.Start Dialogue Event`))

(event `Start Dialogue Event`
  (bind _dialogueui (`self.DialogueUI`))
  (bind _dialogueui_2 (`self.DialogueUI`))
  (bind _dialogueui_3 (`self.DialogueUI`))
  (bind _returnvalue (+ (`/Game/Level_Game/WBP_Dialogue.DialogueTextRow` (`self.DialogueUI`)) 1))
  (bind _returnvalue_2 (+ (`/Game/Level_Game/WBP_Dialogue.DialogueTextRow` (`self.DialogueUI`)) 1))
  (if (not (and (>= _returnvalue_2 11) (<= _returnvalue_2 18)))
    (switch `int` _returnvalue_2
      (:`0`
        _)
      (:`1`
        _)
      (:`2`
        _)
      (:`3`
        _)
      (:`4`
        (`GameplayStatics.PlaySound2D` "/Game/Level_Game/Sound/Roulement_de_tambour.Roulement_de_tambour" 1.0 1.0 0.0 null null))
      (:`5`
        (`GameplayStatics.PlaySound2D` "/Game/Level_Game/Sound/Roulement_de_tambour.Roulement_de_tambour" 1.0 1.0 0.0 null null))
      (:`6`
        (`GameplayStatics.PlaySound2D` "/Game/Level_Game/Sound/Roulement_Chute.Roulement_Chute" 1.0 1.0 0.0 null null))
      (:`7`
        (`GameplayStatics.PlaySound2D` "/Game/Level_Game/Sound/Crickets.Crickets" 1.0 1.0 0.0 null null))
      (:`8`
        _)
      (:`9`
        _)
      (:`10`
        (`GameplayStatics.PlaySound2D` "/Game/Level_Game/Sound/Crickets.Crickets" 1.0 1.0 0.0 null null))))
  (switch `int` (`|GetArrayItem` (`self.Order Arr`) _returnvalue_2)
    (:`0`
      (`/Game/Level_Game/WBP_Dialogue.Hide / Display PP Image` _dialogueui_2 (`/Game/Level_Game/WBP_Dialogue.PPBoss` (`self.DialogueUI`)) false)
      (`/Game/Level_Game/WBP_Dialogue.Hide / Display PP Image` _dialogueui_2 (`/Game/Level_Game/WBP_Dialogue.PPSlime` (`self.DialogueUI`)) true))
    (:`1`
      (`/Game/Level_Game/WBP_Dialogue.Hide / Display PP Image` _dialogueui_3 (`/Game/Level_Game/WBP_Dialogue.PPBoss` (`self.DialogueUI`)) true)
      (`/Game/Level_Game/WBP_Dialogue.Hide / Display PP Image` _dialogueui_3 (`/Game/Level_Game/WBP_Dialogue.PPSlime` (`self.DialogueUI`)) false))
    (:`2`
      (`/Game/Level_Game/WBP_Dialogue.Hide / Display PP Image` _dialogueui (`/Game/Level_Game/WBP_Dialogue.PPBoss` (`self.DialogueUI`)) false)
      (`/Game/Level_Game/WBP_Dialogue.Hide / Display PP Image` _dialogueui (`/Game/Level_Game/WBP_Dialogue.PPSlime` (`self.DialogueUI`)) false)))
  (`/Engine/EditorBlueprintResources/StandardMacros.DoOnce` false :!label _label
    (:`Completed`
      (set `/Game/Level_Game/WBP_Dialogue.DialogueText` (`self.NPCText`) (`self.DialogueUI`))
      (`Widget.SetVisibility` (`/Game/Level_Game/WBP_Dialogue.Talk` (`self.DialogueUI`)) "Visible")
      (if (> _returnvalue (- (`KismetArrayLibrary.Array_Length` (`self.NPCText`)) 1))
        (`Widget.RemoveFromParent` (`self.DialogueUI`))
        (if (>= (`/Game/Level_Game/WBP_Dialogue.DialogueTextRow` (`self.DialogueUI`)) 17)
          (`GameplayStatics.OpenLevelBySoftObjectPtr` "/Game/Level_Game/Map.Map")
          (else
            (`self.Reset Dialogue`)))
        (else
          (set `/Game/Level_Game/WBP_Dialogue.DialogueTextRow` _returnvalue (`self.DialogueUI`))
          (`self.Reset Dialogue`))))))

(event `Reset Dialogue`
  (goto _label :!via `Reset`))

(fn `UserConstructionScript`)