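; BP_zone_end is a trigger volume that shows an end-zone UI while the player stands inside it.
; When a BP_ThirdPersonCharacter enters the Box, it creates a WBP_End_Zone widget for that character's player controller, adds it to the viewport and plays its Anim.
; When the character leaves the Box, the stored widget is removed from its parent.
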(event `self.Box.OnComponentBeginOverlap`
  (params (OverlappedComponent :type "PrimitiveComponent Object Reference") (OtherActor :type "Actor Object Reference") (OtherComp :type "PrimitiveComponent Object Reference") (OtherBodyIndex :type Integer) (bFromSweep :type Boolean) (SweepResult :type "HitResult Structure (by ref)"))
  (bind _asbp_third_person_character (cast `/Game/ThirdPerson/Blueprints/BP_ThirdPersonCharacter` OtherActor))
  (bind _asplayer_controller (cast `PlayerController` (`Pawn.GetController` _asbp_third_person_character)))
  (bind _returnvalue (`|CreateWidget` "/Game/Level_Game/WBP_End_Zone.WBP_End_Zone_C" _asplayer_controller))
  (bind _output_get (set `self.WBP_Ref` _returnvalue))
  (`UserWidget.AddToViewport` _output_get 0)
  (`/Game/Level_Game/WBP_End_Zone.anim` _output_get))

(event `self.Box.OnComponentEndOverlap`
  (params (OverlappedComponent :type "PrimitiveComponent Object Reference") (OtherActor :type "Actor Object Reference") (OtherComp :type "PrimitiveComponent Object Reference") (OtherBodyIndex :type Integer))
  (cast `/Game/ThirdPerson/Blueprints/BP_ThirdPersonCharacter` OtherActor)
  (`Widget.RemoveFromParent` (`self.WBP_Ref`)))

(fn `UserConstructionScript`)